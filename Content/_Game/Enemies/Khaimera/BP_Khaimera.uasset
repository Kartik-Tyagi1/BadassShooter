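; Khaimera enemy Blueprint that handles the enemy's UI feedback: a health bar widget and floating hit numbers.
; On BeginPlay it links the health bar to itself and hides it; show and hide events toggle visibility, with showing also calling the parent implementation.
; Each hit spawns an animated damage widget with a headshot flag at the projected screen position, registered through StoreHitNumber with its world location.
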(event `self.ReceiveBeginPlay`
  (bind _asbp_enemy_health_bar (cast `/Game/_Game/HUD/BP_EnemyHealthBar` (`WidgetComponent.GetUserWidgetObject` (`self.EnemyHealthBar`))))
  (set `/Game/_Game/HUD/BP_EnemyHealthBar.Enemy` self _asbp_enemy_health_bar)
  (`Widget.SetVisibility` (`WidgetComponent.GetUserWidgetObject` (`self.EnemyHealthBar`)) "Hidden"))

(event `self.ShowHealthBar`
  (`Widget.SetVisibility` (`WidgetComponent.GetUserWidgetObject` (`self.EnemyHealthBar`)) "Visible")
  (`parent.ShowHealthBar`))

(event `self.HideHealthBar`
  (`Widget.SetVisibility` (`WidgetComponent.GetUserWidgetObject` (`self.EnemyHealthBar`)) "Hidden"))

(event `self.ShowHitNumbers`
  (params (Damage :type "Float (single-precision)") (HitLocation :type "Vector Structure") (bIsHeadShot :type Boolean))
  (bind _returnvalue (`|CreateWidget` "/Game/_Game/HUD/BP_HitNumbers.BP_HitNumbers_C"))
  (`UserWidget.AddToViewport` _returnvalue 0)
  (`UserWidget.SetPositionInViewport` _returnvalue (`GameplayStatics.ProjectWorldToScreen` (`GameplayStatics.GetPlayerController` 0) HitLocation) true)
  (`self.StoreHitNumber` _returnvalue HitLocation)
  (set `/Game/_Game/HUD/BP_HitNumbers.HitText` (`KismetTextLibrary.Conv_DoubleToText` Damage "HalfToEven") _returnvalue)
  (set `/Game/_Game/HUD/BP_HitNumbers.IsHeadshot` bIsHeadShot _returnvalue)
  (`UserWidget.PlayAnimation` _returnvalue (`/Game/_Game/HUD/BP_HitNumbers.HitNumberTextAnim` _returnvalue) 0.0 1 "Forward" 1.0 false))

(fn `UserConstructionScript`)