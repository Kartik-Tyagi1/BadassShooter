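; HUD class that draws a dynamic four-piece crosshair at screen center while the shooter character is in combat pose.
; Each DrawHUD reads the character's spread multiplier and scales it by a maximum spread to push the top, bottom, left and right textures outward.
; DrawHUD re-acquires the character reference from the player pawn whenever it is invalid.
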(event `self.ReceiveBeginPlay`
  ;[1 1 1] Reference to Shooter Character
  (`/Engine/EditorBlueprintResources/StandardMacros.IsValid` (`self.ShooterCharacter`)
    (:`Is Valid`
      (bind _asbp_shooter_character (cast `/Game/_Game/Character/BP_ShooterCharacter` (`GameplayStatics.GetPlayerPawn` 0)))
      (set `self.ShooterCharacter` _asbp_shooter_character))))

(event `self.ReceiveDrawHUD`
  (params (SizeX :type Integer) (SizeY :type Integer))
  (bind (_crosshair_location_x _crosshair_location_y) (`KismetMathLibrary.BreakVector2D` (`self.Crosshair Location`)))
  (bind (_crosshair_location_x_2 _crosshair_location_y_2) (`KismetMathLibrary.BreakVector2D` (`self.Crosshair Location`)))
  (bind (_crosshair_location_x_3 _crosshair_location_y_3) (`KismetMathLibrary.BreakVector2D` (`self.Crosshair Location`)))
  (bind (_crosshair_location_x_4 _crosshair_location_y_4) (`KismetMathLibrary.BreakVector2D` (`self.Crosshair Location`)))
  (bind _returnvalue (/ (`self.Crosshair Size`) 2.0))
  (bind _returnvalue_2 (/ (`self.Crosshair Size`) 2.0))
  (bind _returnvalue_3 (/ (`self.Crosshair Size`) 2.0))
  (bind _returnvalue_4 (/ (`self.Crosshair Size`) 2.0))
  (bind _output_get (set `self.Screen Center` (`KismetMathLibrary.MakeVector2D` (`KismetMathLibrary.Conv_IntToDouble` (/ SizeX 2)) (`KismetMathLibrary.Conv_IntToDouble` (/ SizeY 2)))))
  ;[1 1 1] Double check Reference to Shooter Character
  (set `self.Crosshair Location` _output_get)
  (`/Engine/EditorBlueprintResources/StandardMacros.IsValid` (`self.ShooterCharacter`)
    (:`Is Valid`
      _)
    (:`Is Not Valid`
      (bind _asbp_shooter_character (cast `/Game/_Game/Character/BP_ShooterCharacter` (`GameplayStatics.GetPlayerPawn` 0)))
      (bind _output_get_2 (set `self.ShooterCharacter` _asbp_shooter_character))))
  ;[1 1 1] Get Crosshair Spread Multiplier
  (set `self.CrosshairSpreadMultiplier` (`ShooterCharacter.GetCrosshairSpreadMultiplier` (`self.ShooterCharacter`)))
  (bind _output_get_3 (set `self.IsInCombatPose` (`ShooterCharacter.GetIsInCombatPose` _output_get_2)))
  (if _output_get_3
    ;[1 1 1] Bottom Crosshair
    (`self.DrawTexture` "/Game/_Game/Assets/Textures/Textures/Crosshairs/Quad_9_Bottom.Quad_9_Bottom" (- _crosshair_location_x_4 _returnvalue) (- (+ _crosshair_location_y_4 (* (`self.CrosshairSpreadMultiplier`) (`self.CrosshairSpreadMax`))) _returnvalue) 64.0 64.0 0.0 0.0 1.0 1.0)
    ;[1 1 1] Top Crosshair
    (`self.DrawTexture` "/Game/_Game/Assets/Textures/Textures/Crosshairs/Quad_9_Top.Quad_9_Top" (- _crosshair_location_x _returnvalue_3) (- (- _crosshair_location_y (* (`self.CrosshairSpreadMultiplier`) (`self.CrosshairSpreadMax`))) _returnvalue_3) 64.0 64.0 0.0 0.0 1.0 1.0)
    ;[1 1 1] Right Crosshair
    (`self.DrawTexture` "/Game/_Game/Assets/Textures/Textures/Crosshairs/Quad_9_Right.Quad_9_Right" (- (+ _crosshair_location_x_2 (* (`self.CrosshairSpreadMultiplier`) (`self.CrosshairSpreadMax`))) _returnvalue_4) (- _crosshair_location_y_2 _returnvalue_4) 64.0 64.0 0.0 0.0 1.0 1.0)
    ;[1 1 1] Left Crosshair
    (`self.DrawTexture` "/Game/_Game/Assets/Textures/Textures/Crosshairs/Quad_9_Left.Quad_9_Left" (- (- _crosshair_location_x_3 (* (`self.CrosshairSpreadMultiplier`) (`self.CrosshairSpreadMax`))) _returnvalue_2) (- _crosshair_location_y_3 _returnvalue_2) 64.0 64.0 0.0 0.0 1.0 1.0)))

(fn `UserConstructionScript`)