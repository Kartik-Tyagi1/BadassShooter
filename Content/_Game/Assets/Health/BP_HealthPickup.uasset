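; BP_HealthPickup is a pickup that restores health to a BP_ShooterCharacter that walks into it.
; Overlapping its PickupSphere casts the other actor to the shooter character and adds HealthAmount to Health, clamped at MaxHealth.
; It then plays the health pickup sound at its location and destroys itself, even if the character was already at full health.
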(event `self.PickupSphere.OnComponentBeginOverlap`
  (params (OverlappedComponent :type "PrimitiveComponent Object Reference") (OtherActor :type "Actor Object Reference") (OtherComp :type "PrimitiveComponent Object Reference") (OtherBodyIndex :type Integer) (bFromSweep :type Boolean) (SweepResult :type "HitResult Structure (by ref)"))
  (bind _asbp_shooter_character (cast `/Game/_Game/Character/BP_ShooterCharacter` OtherActor))
  (bind _returnvalue (+ (`ShooterCharacter.Health` _asbp_shooter_character) (`self.HealthAmount`)))
  (bind _maxhealth (`ShooterCharacter.MaxHealth` _asbp_shooter_character))
  (if (> _returnvalue _maxhealth)
    (set `ShooterCharacter.Health` _maxhealth _asbp_shooter_character)
    (else
      (set `ShooterCharacter.Health` _returnvalue _asbp_shooter_character)))
  (`GameplayStatics.PlaySoundAtLocation` "/Game/_Game/Assets/Sounds/Pickups/sw_Pickup_Health.sw_Pickup_Health" (`self.K2_GetActorLocation`) (struct) 1.0 1.0 0.0 null null null)
  (`self.K2_DestroyActor`))

(fn `UserConstructionScript`)